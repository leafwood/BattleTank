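; Player-controllable tank Blueprint that delegates aiming, firing and movement to its AimingComp and TankMovement components.
; On BeginPlay it passes the barrel to the aiming component and the body to the movement component.
; Input drives firing, forward and turn intents, while camera axes rotate the Azimuth component for yaw and the SpringArm for pitch.
; Hits on TankBody call its Compound function.
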(event OnComponentHit(TankBody)
  (params (HitComponent :type Primitive%20Component%20Object%20Reference) (OtherActor :type Actor%20Object%20Reference) (OtherComp :type Primitive%20Component%20Object%20Reference) (NormalImpulse :type Vector :default "0, 0, 0") (Hit :type Hit%20Result%20Structure%20%28by%20ref%29))
  (Class|TankBody|Compound (Variables|Default|GetTankBody)))

(event EventBeginPlay
  (Class|AimingComponent|InitializeAimComp (Variables|Default|GetAimingComp) (Variables|Default|GetTankBarrel))
  (Class|TankMovementComponent|Initialize (Variables|Default|GetTankMovement) (Variables|Default|GetTankBody)))

(event Collision|EventActorBeginOverlap
  (params (OtherActor :type Actor%20Object%20Reference)))

(event EventTick
  (params (DeltaSeconds :type Float%20%28single-precision%29)))

(event Input|ActionEvents|InputActionFire
  (params (Key :type Key%20Structure :default "None"))
  ;[1 1 1] input
  (:Pressed
    (Class|AimingComponent|Fire (Variables|Default|GetAimingComp))))

(event Input|AxisEvents|InputAxisRightTrack
  (params (AxisValue :type Float%20%28single-precision%29))
  ;[1 1 1] input
  (Class|TankMovementComponent|IntendTurnRight (Variables|Default|GetTankMovement) AxisValue))

(event Input|AxisEvents|InputAxisMoveForward
  (params (AxisValue :type Float%20%28single-precision%29))
  ;[1 1 1] input
  (Class|TankMovementComponent|IntendMoveForward (Variables|Default|GetTankMovement) AxisValue))

(event Input|AxisEvents|InputAxisAimAzimuth
  (params (AxisValue :type Float%20%28single-precision%29))
  ;[1 1 1] Camera Binding
  (Transformation|AddLocalRotation (Variables|Default|GetAzimuth) (Math|Rotator|MakeRotator 0.0 0.0 AxisValue) false false))

(event Input|AxisEvents|InputAxisAltitude
  (params (AxisValue :type Float%20%28single-precision%29))
  ;[1 1 1] Camera Binding
  (Transformation|AddLocalRotation (Variables|Default|GetSpringArm) (Math|Rotator|MakeRotator 0.0 AxisValue 0.0) false false))

(fn ConstructionScript)